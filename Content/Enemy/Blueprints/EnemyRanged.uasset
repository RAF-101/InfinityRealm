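; EnemyRanged is a ranged enemy that turns toward the player and fires EnemyProjectile actors.
; BeginPlay caches the player character, then starts self-recalling Delay loops for shooting and facing instead of using Tick.
; A range check polls until the player is close, then sets ShouldFollow, which stays set as the range check stops.
; That flag enables interpolated yaw tracking and periodic projectile spawns ahead of the enemy.
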(event Custom|Shoot%20Player
  (bind _returnvalue (Transformation|GetActorRotation))
  ;[1 1 1] Shoot at player
  (if (Variables|Default|GetShould%20Follow%20)
    (Development|PrintString "in Range")
    (Game|SpawnActorfromClass "/Game/Enemy/Blueprints/EnemyProjectile.EnemyProjectile_C" (Math|Transform|MakeTransform (+ (Transformation|GetActorLocation) (* (Math|Vector|GetForwardVector _returnvalue) (Variables|Default|GetDistance%20of%20spawning))) _returnvalue) "AdjustIfPossibleButAlwaysSpawn" 0 0)
    (Utilities|FlowControl|Delay 5.0))
  (Utilities|FlowControl|Delay 0.2)
  (CallFunction|ShootPlayer))

(event Custom|Face%20Player
  ;[1 1 1] Facing Player
  (if (Variables|Default|GetShould%20Follow%20)
    (Transformation|SetActorRotation (Math|Rotator|MakeRotator 0.0 0.0 (.yaw (Math|Interpolation|RInterpTo (Transformation|GetActorRotation) (Math|Rotator|FindLookatRotation (Transformation|GetActorLocation) (Transformation|GetActorLocation (Variables|Default|GetPlayer%20Reference))) (Utilities|Time|GetWorldDeltaSeconds) 2e+01))))
    (Utilities|FlowControl|Delay 0.001)
    (CallFunction|FacePlayer)
    (else
      (CallFunction|ShouldRotateEvent))))

(event Custom|Should%20Rotate%20Event
  ;[1 1 1] Should it face player
  (if (<= (Transformation|GetDistanceTo (Variables|Default|GetPlayer%20Reference)) (Variables|Default|GetRange))
    (Variables|Default|SetShould%20Follow%20 true)
    (CallFunction|FacePlayer)
    (else
      (Variables|Default|SetShould%20Follow%20 false)
      (Utilities|FlowControl|Delay 0.001)
      (CallFunction|ShouldRotateEvent))))

(event EventBeginPlay
  (bind _asbp_top_down_character (Utilities|Casting|CastToBP_TopDownCharacter (Game|GetPlayerCharacter 0)))
  (Variables|Default|SetPlayer%20Reference _asbp_top_down_character)
  (Utilities|FlowControl|Sequence
    (:then_0
      (CallFunction|ShootPlayer))
    (:then_1
      (CallFunction|FacePlayer))))

(fn ConstructionScript)