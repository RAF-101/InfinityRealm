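; Enemy pawn that follows the top-down player character while it is within SeeDistance.
; On BeginPlay it caches the player reference and starts the recursive GoToPlayer event.
; Each pass issues an AIMoveTo at the player when in range, or at itself otherwise, and repeats after a short delay without waiting for the move to finish.
; Detection is a distance check only.
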(event Custom|Go%20to%20Player
  (if (<= (Transformation|GetDistanceTo (Variables|Default|GetPlayer%20Reference)) (Variables|Default|GetSee%20Distance))
    (AI|AIMoveTo self "0, 0, 0" (Variables|Default|GetPlayer%20Reference) 5.0 false
      (:then
        _))
    (else
      (AI|AIMoveTo self "0, 0, 0" self 5.0 false
        (:then
          _))))
  (Utilities|FlowControl|Delay 0.2)
  (CallFunction|GotoPlayer))

(event EventBeginPlay
  (bind _asbp_top_down_character (Utilities|Casting|CastToBP_TopDownCharacter (Game|GetPlayerCharacter 0)))
  (Variables|Default|SetPlayer%20Reference _asbp_top_down_character)
  (CallFunction|GotoPlayer))

(fn ConstructionScript)