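; Enemy1 is an enemy that chases the top-down player character while it is within sight distance.
; On BeginPlay it caches the player as BP_TopDownCharacter, then starts a self-repeating check every 0.2 seconds.
; Each check uses AI MoveTo toward the player when close, or targets itself when far, and prints a Close or Far debug message.
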(event Custom|Go%20to%20Player
  (if (<= (Transformation|GetDistanceTo (Variables|Default|GetPlayer%20Reference)) (Variables|Default|GetSee%20Distance))
    (Development|PrintText "Close" true true "(R=0.000000,G=0.660000,B=1.000000,A=1.000000)" 0.2)
    (AI|AIMoveTo self "0, 0, 0" (Variables|Default|GetPlayer%20Reference) 5.0 false
      (:then
        _))
    (else
      (Development|PrintText "Far" true true "(R=1.000000,G=0.027614,B=0.000000,A=1.000000)" 0.2)
      (AI|AIMoveTo self "0, 0, 0" self 5.0 false
        (:then
          _))))
  (Utilities|FlowControl|Delay 0.2)
  (CallFunction|GotoPlayer))

(event EventBeginPlay
  (bind _asbp_top_down_character (Utilities|Casting|CastToBP_TopDownCharacter (Game|GetPlayerCharacter 0)))
  (Variables|Default|SetPlayer%20Reference _asbp_top_down_character)
  (CallFunction|GotoPlayer))

(fn ConstructionScript)